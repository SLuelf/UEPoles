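; Learning Agents interactor for a cart-pole balancing agent, defining what each BP_Cart agent observes and how it acts.
; Observations form a struct of scaled floats: cart position relative to the rail and velocity along Y, plus pole roll angle and X angular velocity.
; The single float action is scaled up and applied to the cart as a physics force along Y.
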(fn `GatherAgentObservation`
  (params (InObservationObject :type "LearningAgentsObservationObject Object Reference") (AgentId :type Integer))
  (returns (OutObservationObjectElement :type "LearningAgentsObservationObjectElement Structure"))
  (locals (ObsActor :type "/Game/BP_Cart Object Reference"))
  (bind _cart (`/Game/BP_Cart.Cart` (`local.ObsActor`)))
  (bind _pole (`/Game/BP_Cart.Pole` (`local.ObsActor`)))
  (set `local.ObsActor` (`self.GetAgent` AgentId "/Game/BP_Cart.BP_Cart_C"))
  (return (`LearningAgentsObservations.MakeStructObservation` (`local.InObservationObject`) (`|MakeMap` "CartPos" (`LearningAgentsObservations.MakeFloatObservation` (`local.InObservationObject`) (- (.y (`SceneComponent.GetSocketLocation` _cart "None")) (.y (`SceneComponent.GetSocketLocation` (`/Game/BP_Cart.Rail` (`local.ObsActor`)) "None"))) 100.0 "CartPosition" false null) "CartVel" (`LearningAgentsObservations.MakeFloatObservation` (`local.InObservationObject`) (.y (`SceneComponent.GetComponentVelocity` _cart)) 200.0 "CartVelocity" false null) "PoleAng" (`LearningAgentsObservations.MakeFloatObservation` (`local.InObservationObject`) (.roll (`SceneComponent.GetSocketRotation` _pole "None")) 1.0 "PoleAngle" false null) "PoleAngVel" (`LearningAgentsObservations.MakeFloatObservation` (`local.InObservationObject`) (.x (`PrimitiveComponent.GetPhysicsAngularVelocityInRadians` _pole "Pole")) 1.0 "PoleAngVelocity" false null) :!type "Name"))))

(fn `PerformAgentAction`
  (params (InActionObject :type "LearningAgentsActionObject Object Reference") (InActionObjectElement :type "LearningAgentsActionObjectElement Structure (by ref)") (AgentId :type Integer))
  (locals (ActActor :type "/Game/BP_Cart Object Reference"))
  (set `local.ActActor` (`self.GetAgent` AgentId "/Game/BP_Cart.BP_Cart_C"))
  (bind _outvalue (`LearningAgentsActions.GetFloatAction` (`local.InActionObject`) (`local.InActionObjectElement`) 300000.0 "CartMove" false null))
  (`PrimitiveComponent.AddForce` (`/Game/BP_Cart.Cart` (`local.ActActor`)) (`KismetMathLibrary.MakeVector` 0.0 _outvalue) "Cart" false)
  (return))

(fn `SpecifyAgentAction`
  (params (InActionSchema :type "LearningAgentsActionSchema Object Reference"))
  (returns (OutActionSchemaElement :type "LearningAgentsActionSchemaElement Structure"))
  (return (`LearningAgentsActions.SpecifyFloatAction` (`local.InActionSchema`) "CartMove")))

(fn `SpecifyAgentObservation`
  (params (InObservationSchema :type "LearningAgentsObservationSchema Object Reference"))
  (returns (OutObservationSchemaElement :type "LearningAgentsObservationSchemaElement Structure"))
  (return (`LearningAgentsObservations.SpecifyStructObservation` (`local.InObservationSchema`) (`|MakeMap` "CartPos" (`LearningAgentsObservations.SpecifyFloatObservation` (`local.InObservationSchema`) "CartPosition") "CartVel" (`LearningAgentsObservations.SpecifyFloatObservation` (`local.InObservationSchema`) "CartVelocity") "PoleAng" (`LearningAgentsObservations.SpecifyFloatObservation` (`local.InObservationSchema`) "PoleAngle") "PoleAngVel" (`LearningAgentsObservations.SpecifyFloatObservation` (`local.InObservationSchema`) "PoleAngVelocity") :!type "Name"))))
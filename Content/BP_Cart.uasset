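; Physics cart-pole actor, with a cart, rail and pole, that serves as a Learning Agents agent.
; On BeginPlay it finds the LearningAgentsManager component on actors tagged for it, registers itself and stores the AgentID, printing an error if none is found.
; ResetCart, not called by live logic here, recenters the cart on the rail and places the pole above with a slight random roll, zeroing cart linear velocity and pole velocities.
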(event `self.ReceiveBeginPlay`
  (bind _outactors (`GameplayStatics.GetAllActorsWithTag` "LearningAgentsManager"))
  (for _array_element _outactors
    (bind _returnvalue (`self.GetComponentByClass` _array_element "/Script/LearningAgents.LearningAgentsManager"))
    (`/Engine/EditorBlueprintResources/StandardMacros.IsValid` _returnvalue
      (:`Is Valid`
        (bind _returnvalue_2 (`LearningAgentsManager.AddAgent` _returnvalue self))
        (set `self.AgentID` _returnvalue_2)
        (set `self.FoundManager` true))))
  (if (not (`self.FoundManager`))
    (`KismetSystemLibrary.PrintString` "Failed to find the manager")))

(event `self.ReceiveTick`
  (params (DeltaSeconds :type "Float (single-precision)")))

(fn `ResetCart`
  (bind _cart (`self.Cart`))
  (bind _pole (`self.Pole`))
  (bind _returnvalue (`SceneComponent.K2_GetComponentLocation` (`self.Rail`)))
  (`SceneComponent.K2_SetWorldLocation` _cart _returnvalue false false)
  (`PrimitiveComponent.SetPhysicsLinearVelocity` _cart (0.0 0.0 0.0) false "Cart")
  (`SceneComponent.K2_SetWorldLocationAndRotation` _pole (`KismetMathLibrary.MakeVector` (.x _returnvalue) (.y _returnvalue) (+ (.z _returnvalue) 250.0)) (`KismetMathLibrary.MakeRotator` (`KismetMathLibrary.RadiansToDegrees` (`KismetMathLibrary.RandomFloatInRange` -0.01 0.01))) false false)
  (`PrimitiveComponent.SetPhysicsAngularVelocityInRadians` _pole (0.0 0.0 0.0) false "Pole")
  (`PrimitiveComponent.SetPhysicsLinearVelocity` _pole (0.0 0.0 0.0) false "Pole"))

(fn `UserConstructionScript`)
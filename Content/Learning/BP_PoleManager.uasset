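; Manager actor that trains cart-pole agents (BP_Cart) with the Learning Agents plugin.
; On BeginPlay it makes every cart tick after itself, then chains interactor, policy, critic and trainer on the LearningAgentsManager, using encoder, policy and decoder network assets.
; It then resets the carts and sets global time dilation to speed up the simulation.
; Each Tick runs training through the trainer.
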(event `self.ReceiveBeginPlay`
  (`|ExecutionSequence`
    (:`then_0`
      (bind _outactors (`GameplayStatics.GetAllActorsOfClass` "/Game/BP_Cart.BP_Cart_C"))
      (bind _output_get (set `self.PoleActors` _outactors))
      (`self.AddTickPrerequisiteActor` _output_get self))
    (:`then_1`
      (bind _returnvalue (`LearningAgentsInteractor.MakeInteractor` (`self.LearningAgentsManager`) "/Game/BP_PoleInteractor.BP_PoleInteractor_C" "PoleInteractor"))
      (set `self.Interactor` _returnvalue))
    (:`then_2`
      (bind _returnvalue_2 (`LearningAgentsPolicy.MakePolicy` (`self.LearningAgentsManager`) (`self.Interactor`) "/Script/LearningAgents.LearningAgentsPolicy" "PolePolicy" "/Game/DA_PoleEncoder.DA_PoleEncoder" "/Game/DA_PolePolicy.DA_PolePolicy" "/Game/DA_PoleDecoder.DA_PoleDecoder" true true true (`self.Policy Settings`)))
      (set `self.Policy` _returnvalue_2))
    (:`then_3`
      (bind _returnvalue_3 (`LearningAgentsCritic.MakeCritic` (`self.LearningAgentsManager`) (`self.Interactor`) (`self.Policy`) "/Script/LearningAgents.LearningAgentsCritic" "PoleCritic" null true (`self.Critic Settings`)))
      (set `self.Critic` _returnvalue_3))
    (:`then_4`
      (bind _returnvalue_4 (`LearningAgentsTrainer.MakeTrainer` (`self.LearningAgentsManager`) (`self.Interactor`) (`self.Policy`) (`self.Critic`) "/Game/BP_PoleTrainer.BP_PoleTrainer_C" "PoleTrainer" (`self.Trainer Settings`)))
      (set `self.Trainer` _returnvalue_4))
    (:`then_5`
      (`/Game/BP_Cart.ResetCart` (`self.PoleActors`)))
    (:`then_6`
      (`GameplayStatics.SetGlobalTimeDilation` 10.0))))

(event `self.ReceiveTick`
  (params (DeltaSeconds :type "Float (single-precision)"))
  (`LearningAgentsTrainer.RunTraining` (`self.Trainer`) (`self.Trainer Training Settings`) (`self.Trainer Game Settings`) (`self.Trainer Path Settings`) true true))

(fn `UserConstructionScript`)
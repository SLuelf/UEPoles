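; BP_PoleTrainer defines the reward, completion and reset logic for training BP_Cart agents at pole balancing, in Learning Agents style.
; Each agent receives a constant reward, so longer episodes earn more.
; An episode terminates when the absolute roll of the cart's Pole, converted to radians, reaches or exceeds a fixed threshold.
; Episode reset is delegated to the cart's ResetCart.
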(fn `GatherAgentCompletion`
  (params (AgentId :type Integer))
  (returns (OutCompletion :type "ELearningAgentsCompletion Enum"))
  (locals (AngleTooBig :type Boolean))
  (`/Engine/EditorBlueprintResources/StandardMacros.CompareFloat` (`KismetMathLibrary.Abs` (`KismetMathLibrary.DegreesToRadians` (.roll (`SceneComponent.GetSocketRotation` (`/Game/BP_Cart.Pole` (`self.GetAgent` AgentId "/Game/BP_Cart.BP_Cart_C")) "None")))) 0.4
    (:`>`
      (set `local.AngleTooBig` true :!label _label))
    (:`==`
      (goto _label))
    (:`<`
      _))
  (return (`LearningAgentsCompletions.MakeCompletionOnCondition` (`local.AngleTooBig`) "Termination" "ConditionCompletion" false null)))

(fn `GatherAgentReward`
  (params (AgentId :type Integer))
  (returns (OutReward :type "Float (single-precision)"))
  (locals (RewardActor :type "/Game/BP_Cart Object Reference"))
  (set `local.RewardActor` (`self.GetAgent` AgentId "/Game/BP_Cart.BP_Cart_C"))
  (return (`LearningAgentsRewards.MakeReward` 1.0 1.0 "Reward" false null)))

(fn `ResetAgentEpisode`
  (params (AgentId :type Integer))
  (`/Game/BP_Cart.ResetCart` (`self.GetAgent` AgentId "/Game/BP_Cart.BP_Cart_C")))